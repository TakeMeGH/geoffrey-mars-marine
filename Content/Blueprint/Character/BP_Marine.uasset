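; Player-controlled marine character for a top-down mouse-aim shooter, with health, death and a kill counter.
; Enhanced Input drives world-axis movement, while each tick a cursor trace smoothly turns the control rotation toward the hit point.
; Holding shoot plays muzzle effects and looping audio while a repeating timer line-traces from the rifle muzzle to apply damage.
; Incoming damage lowers clamped health; at zero, firing stops and the death flag blocks movement, aiming and shooting.
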(event `self.ReceiveBeginPlay`
  (`EnhancedInputSubsystemInterface.AddMappingContext` (pcsubsystem `EnhancedInputLocalPlayerSubsystem` (`GameplayStatics.GetPlayerController` 0)) "/Game/Input/IMC_Player.IMC_Player" 0 (struct))
  (set `PlayerController.bShowMouseCursor` true (`GameplayStatics.GetPlayerController` 0))
  (bind _returnvalue (`|CreateWidget` "/Game/UI/WBP_PlayerHUD.WBP_PlayerHUD_C" null self))
  (`UserWidget.AddToViewport` _returnvalue 0)
  (set `self.CurrentHealth` (`self.MaxHealth`)))

(event `EnhancedInput|/Game/Input/IA_ForwardBackwards`
  (params (ActionValue :type "Float (double-precision)") (ElapsedSeconds :type "Float (double-precision)") (TriggeredSeconds :type "Float (double-precision)") (InputAction :type "InputAction Object Reference" :default "/Game/Input/IA_ForwardBackwards.IA_ForwardBackwards"))
  (:`Triggered`
    (if (`self.IsAlive`)
      (`self.AddMovementInput` (1.0 0.0 0.0) ActionValue))))

(event `EnhancedInput|/Game/Input/IA_Shoot`
  (params (ActionValue :type Boolean) (ElapsedSeconds :type "Float (double-precision)") (TriggeredSeconds :type "Float (double-precision)") (InputAction :type "InputAction Object Reference" :default "/Game/Input/IA_Shoot.IA_Shoot"))
  (:`Started`
    (`self.StartShooting`))
  (:`Completed`
    (`self.StopShooting`)))

(event `EnhancedInput|/Game/Input/IA_LeftRight`
  (params (ActionValue :type "Float (double-precision)") (ElapsedSeconds :type "Float (double-precision)") (TriggeredSeconds :type "Float (double-precision)") (InputAction :type "InputAction Object Reference" :default "/Game/Input/IA_LeftRight.IA_LeftRight"))
  (:`Triggered`
    (if (`self.IsAlive`)
      (`self.AddMovementInput` (0.0 1.0 0.0) ActionValue))))

(event `self.ReceiveTick`
  (params (DeltaSeconds :type "Float (single-precision)"))
  (`self.UpdatePlayerAIM`))

(event `self.ReceiveAnyDamage`
  (params (Damage :type "Float (single-precision)") (DamageType :type "DamageType Object Reference") (InstigatedBy :type "Controller Object Reference") (DamageCauser :type "Actor Object Reference"))
  (`self.DecreaseHealth` Damage)
  (if (== (`self.CurrentHealth`) 0.0)
    (`self.StopShooting`)
    (set `self.IsDead` true)))

(event `IncreaseKillCount`
  (`/Engine/EditorBlueprintResources/StandardMacros.IncrementInt` (`self.KillCount`)))

(fn `DecreaseHealth`
  (params (Damage :type "Float (double-precision)"))
  (set `self.CurrentHealth` (`KismetMathLibrary.FClamp` (- (`self.CurrentHealth`) Damage) 0.0 (`self.MaxHealth`))))

(fn `GetWeaponTraceEndLocation`
  (returns (ReturnValue :type "Vector Structure"))
  (return (+ (`self.GetWeaponTraceStartLocation`) (* (`self.GetActorForwardVector`) (`self.WeaponRange`)))))

(fn `GetWeaponTraceStartLocation`
  (returns (ReturnValue :type "Vector Structure"))
  (return (`SceneComponent.GetSocketLocation` (`self.Rifle`) "MuzzleFlashSocket")))

(fn `IsAlive`
  (returns (ReturnValue :type Boolean))
  (return (not (`self.IsDead`))))

(fn `StartShooting`
  (if (`self.IsAlive`)
    (`ActorComponent.Activate` (`self.P_AssaultRifle_MF`) false)
    (bind _returnvalue (`GameplayStatics.SpawnSound2D` "/Game/Sounds/Weapon_AssaultRifle/Stereo/AssultRifle_ShootLoop.AssultRifle_ShootLoop" 1.0 1.0 0.0 null))
    (set `self.ShootingSound` _returnvalue)
    (`self.WeaponTrace`)
    (`KismetSystemLibrary.K2_SetTimer` null "WeaponTrace" (`self.FireRate`) true)))

(fn `StopShooting`
  (bind _shootingsound (`self.ShootingSound`))
  (if (`self.IsAlive`)
    (`ActorComponent.Deactivate` (`self.P_AssaultRifle_MF`))
    (`/Engine/EditorBlueprintResources/StandardMacros.IsValid` _shootingsound
      (:`Is Valid`
        (`AudioComponent.Stop` _shootingsound))
      (:`Is Not Valid`
        _))
    (`GameplayStatics.SpawnSound2D` "/Game/Sounds/Weapon_AssaultRifle/Stereo/AssultRifle_ShootEnd.AssultRifle_ShootEnd" 1.0 1.0 0.0 null)
    (`KismetSystemLibrary.K2_ClearTimer` null "WeaponTrace")))

(fn `UpdatePlayerAIM`
  (bind _returnvalue (`GameplayStatics.GetPlayerController` 0))
  (bind (_locationx _locationy) (`PlayerController.GetMousePosition` _returnvalue))
  (bind (_worldposition _worlddirection) (`GameplayStatics.DeprojectScreenToWorld` _returnvalue (`KismetMathLibrary.MakeVector2D` _locationx _locationy)))
  (if (`self.IsAlive`)
    (bind _outhit (`KismetSystemLibrary.LineTraceSingle` _worldposition (+ _worldposition (* _worlddirection 20000.0)) "TraceTypeQuery1"))
    (`Controller.SetControlRotation` (`GameplayStatics.GetPlayerController` 0) (`KismetMathLibrary.RInterpTo` (`Controller.GetControlRotation` (`GameplayStatics.GetPlayerController` 0)) (`KismetMathLibrary.FindLookAtRotation` (`self.K2_GetActorLocation`) (`.Location` (`GameplayStatics.BreakHitResult` _outhit))) (`GameplayStatics.GetWorldDeltaSeconds`) (`self.RotationSpeed`)))))

(fn `UserConstructionScript`)

(fn `WeaponTrace`
  (bind _outhit (`KismetSystemLibrary.LineTraceSingle` (`self.GetWeaponTraceStartLocation`) (`self.GetWeaponTraceEndLocation`) "TraceTypeQuery1"))
  (bind (_bblockinghit _binitialoverlap _time _distance _location _impactpoint _normal _impactnormal _physmat _hitactor) (`GameplayStatics.BreakHitResult` _outhit))
  (if _bblockinghit
    (`GameplayStatics.ApplyDamage` _hitactor (`self.Base Damage`))))