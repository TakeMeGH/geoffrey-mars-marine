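; BP_Alien is an enemy alien character that chases the player and attacks at close range.
; From BeginPlay it runs AIMoveTo toward the player pawn, repeating after a short delay each time a move succeeds.
; Tick checks whether the player is within AttackRange and no attack montage is playing, then deactivates CharacterMovement, plays the attack montage, and reactivates movement when it completes.
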(event `self.ReceiveBeginPlay`
  (`|AIMoveTo` self (0.0 0.0 0.0) (`GameplayStatics.GetPlayerPawn` 0) :!label _label
    (:`OnSuccess`
      (`KismetSystemLibrary.Delay` 0.4)
      (goto _label))))

(event `self.ReceiveTick`
  (params (DeltaSeconds :type "Float (single-precision)"))
  (if (and (`self.IsWithinAttackRange`) (not (`self.IsAttackMontagePlaying`)))
    (`ActorComponent.Deactivate` (`self.CharacterMovement`))
    (`|PlayMontage` (`self.Mesh`) "/Game/Characters/Enemy_Great_Spider/Animations/Alien_Attack_Montage.Alien_Attack_Montage"
      (:`OnCompleted`
        (`ActorComponent.Activate` (`self.CharacterMovement`) false)))))

(fn `IsAttackMontagePlaying`
  (returns (ReturnValue :type Boolean))
  (return (`AnimInstance.Montage_IsPlaying` (`SkeletalMeshComponent.GetAnimInstance` (`self.Mesh`)) "/Game/Characters/Enemy_Great_Spider/Animations/Alien_Attack_Montage.Alien_Attack_Montage")))

(fn `IsWithinAttackRange`
  (returns (ReturnValue :type Boolean))
  (return (< (`self.GetDistanceTo` (`GameplayStatics.GetPlayerPawn` 0)) (`self.AttackRange`))))

(fn `UserConstructionScript`)